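; Bomb component that blows up its owning actor after a delay, destroying nearby destructible objects.
; BeginPlay starts a timer using ExplosionDelayTime that calls Explode.
; Explode checks every actor overlapping BombAOE for a Destructible_Component and calls DestroyViaBomb on it.
; It then clears the timer and destroys the owner.
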(event EventBeginPlay
  (bind _returnvalue (Utilities|Time|SetTimerbyFunctionName 0 "Explode" (Variables|Default|GetExplosionDelayTime)))
  (Variables|Default|SetDelayTimerHandle _returnvalue))

(event EventTick
  (params (DeltaSeconds :type Float%20%28single-precision%29)))

(fn Explode
  (for _array_element (Collision|GetOverlappingActors (Variables|Default|GetBombAOE) 0 :!class /Script/Engine.PrimitiveComponent)
    ;[1 1 1] Destroy destructible objects
    (Utilities|IsValid (Actor|GetComponentbyClass _array_element "/Script/BombermanMechanics.Destructible_Component")
      (:Is%20Valid
        (Class|DestructibleComponent|DestroyViaBomb (Actor|GetComponentbyClass _array_element "/Script/BombermanMechanics.Destructible_Component")))))
  ;[1 1 1] Clean up self
  (Utilities|Time|ClearandInvalidateTimerbyHandle (Variables|Default|GetDelayTimerHandle))
  (Actor|DestroyActor (Components|GetOwner)))