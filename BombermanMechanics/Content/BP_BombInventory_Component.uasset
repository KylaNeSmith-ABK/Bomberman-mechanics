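; Actor component that gives its owner a bomb inventory, tracking how many bombs it holds and letting it drop them.
; AddBomb increments BombCount, and HasBomb reports whether the count is above zero.
; DropBomb checks HasBomb, then spawns an actor at the owner's transform and decrements the count.
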(event EventBeginPlay)

(event EventTick
  (params (DeltaSeconds :type Float%20%28single-precision%29)))

(fn DropBomb
  (bind _bhasbomb (CallFunction|HasBomb))
  (if _bhasbomb
    (Game|SpawnActorfromClass "/Game/ThirdPerson/Blueprints/BP_Bomb.BP_Bomb_C" (Transformation|GetActorTransform (Components|GetOwner)) "Undefined" 0 0)
    (Variables|Default|SetBombCount (- (Variables|Default|GetBombCount) 1))))

(fn HasBomb
  (return (> (Variables|Default|GetBombCount) 0)))

(fn AddBomb
  (Variables|Default|SetBombCount (+ (Variables|Default|GetBombCount) 1)))